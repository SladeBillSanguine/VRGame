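; VR sliding tile puzzle that, when solved, plays a lock sound, flags a key and updates a MoveableDrawer's lock state.
; The construction script builds a grid of box slots and textured tiles with one gap, optionally shuffles it and scales it to the desired size.
; Grabbing picks the tile nearest the motion controller and slides it via timeline into an empty neighboring slot.
; Overlap queries find that slot and check for the solved layout during movement.
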(event `self.ReceiveTick`
  (params (DeltaSeconds :type "Float (single-precision)")))

(event `SearchFor GrabMesh`
  (bind _returnvalue (`SceneComponent.K2_GetComponentLocation` (`self.Motion Controller`)))
  (`self.Motion Controller`
    (:`then`
      (for _array_element (`self.MeshTrackingList`)
        (`self.DraggedMesh`
          (:`then`
            (if (<= (`KismetMathLibrary.Vector_Distance` (`SceneComponent.K2_GetComponentLocation` _array_element) _returnvalue) (`KismetMathLibrary.Vector_Distance` (`SceneComponent.K2_GetComponentLocation` (`self.DraggedMesh`)) _returnvalue))
              (set `self.DraggedMesh` _array_element)))
          (:`else`
            (set `self.DraggedMesh` _array_element))))
      (`self.MeshGrabbed`))
    (:`else`)))

(event `self.ReceiveBeginPlay`)

(event `MeshGrabbed`
  ;[1 1 1] Grab Version(aktuell)
  (`self.DraggedMesh`
    (:`then`
      (bind _neightbours (`self.GetNeightbours`))
      (`KismetSystemLibrary.PrintText` "Neightbours")
      (for _array_element _neightbours
        (`KismetSystemLibrary.PrintString` (`KismetSystemLibrary.GetDisplayName` _array_element)))
      (`self.GetMoveTo` _neightbours)
      (bind _movetotarget (`self.MoveToTarget`)
        (:`then`
          (`KismetSystemLibrary.PrintText` "Movetotarget")
          (`KismetSystemLibrary.PrintString` (`KismetSystemLibrary.GetDisplayName` _movetotarget))
          (`KismetSystemLibrary.PrintText` "DraggedMesh")
          (`KismetSystemLibrary.PrintString` (`KismetSystemLibrary.GetDisplayName` (`self.DraggedMesh`)))
          (`self.TriggeredMove`))
        (:`else`)))
    (:`else`)))

(event `MeshClicked`
  (params (TouchedComponent :type "PrimitiveComponent Object Reference") (ButtonPressed :type "Key Structure" :default "None"))
  (bind _draggedmesh (`self.DraggedMesh`))
  ;[1 1 1] ONClicked Version
  (bind _output_get (set `self.DraggedMesh` TouchedComponent))
  (add `PrimitiveComponent.OnClicked` _output_get (delegate `MeshClicked`))
  (`KismetSystemLibrary.PrintString` "Dragged Mesh:")
  (`KismetSystemLibrary.PrintString` (`KismetSystemLibrary.GetDisplayName` _output_get))
  (bind _neightbours (`self.GetNeightbours`))
  (`KismetSystemLibrary.PrintText` "Neightbours")
  (for (_ _array_index) _neightbours
    (`KismetSystemLibrary.PrintString` (`KismetStringLibrary.Conv_IntToString` _array_index)))
  (`self.GetMoveTo` _neightbours)
  (bind _movetotarget (`self.MoveToTarget`)
    (:`then`
      (`KismetSystemLibrary.PrintText` "Movetotarget")
      (`KismetSystemLibrary.PrintString` (`KismetSystemLibrary.GetDisplayName` _movetotarget))
      (set `self.MoveToStart` (`SceneComponent.RelativeLocation` _draggedmesh))
      (`KismetSystemLibrary.PrintText` "DraggedMesh")
      (`KismetSystemLibrary.PrintString` (`KismetSystemLibrary.GetDisplayName` _draggedmesh))
      (`self.TriggeredMove`))
    (:`else`
      (set `self.ObjectMoving` false))))

(event `TriggeredMove`
  (if (`self.In Action`)
    (`KismetSystemLibrary.PrintString` "Doesnt Let Object Move")
    (else
      (`KismetSystemLibrary.PrintString` "Obejct Moving True")
      (set `self.ObjectMoving` true)
      (set `self.In Action` true)
      (set `self.MoveToStart` (`SceneComponent.RelativeLocation` (`self.DraggedMesh`)))
      (bind (_direction _newtrack_2) (`Timeline|Move` :!via `PlayFromStart`)
        (:`Update`
          (`SceneComponent.K2_SetRelativeLocation` (`self.DraggedMesh`) (`KismetMathLibrary.VLerp` (`self.MoveToStart`) (`SceneComponent.RelativeLocation` (`self.MoveToTarget`)) _newtrack_2) true false)
          (bind _solved_ (`self.IsSolved?`))
          (if _solved_
            (`KismetSystemLibrary.PrintString` "Moveable Drawer Active")
            (`GameplayStatics.PlaySound2D` "/Game/Eigenarbeit/Assets/Stuff/Sound/Sound/mixkit-door-key-in-door-lock-2842.mixkit-door-key-in-door-lock-2842" 1.0 1.0 0.0 null null) ; Open
            (bind _askey_1 (cast `/Game/Eigenarbeit/BP/Ende1/Key1` (`self.Key`)))
            (`/Game/Eigenarbeit/BP/Ende1/Key1.SetTrue` _askey_1)
            (bind _asmoveable_drawer (cast `/Game/Eigenarbeit/BP/Ende1/MoveableDrawer` (`self.Actor`)))
            (`/Game/Eigenarbeit/BP/Ende1/MoveableDrawer.Set Locked State` _asmoveable_drawer _solved_)))
        (:`Finished`
          (`KismetSystemLibrary.PrintString` "Is Being Grabbed and Obeject Moving Reseted")
          (set `self.In Action` false)
          (set `self.ObjectMoving` false))))))

(event `/Game/Eigenarbeit/BP/Ende1/GrabInterface.Grab`
  (params (MotionController :type "MotionControllerComponent Object Reference"))
  ;[1 1 1] Grab And Release
  (set `self.Motion Controller` MotionController)
  (if (not (`self.ObjectMoving`))
    (`self.SearchFor GrabMesh`)))

(event `/Game/Eigenarbeit/BP/Ende1/GrabInterface.Release`
  (params (MotionController :type "MotionControllerComponent Object Reference"))
  ;[1 1 1] Grab And Release
  (if (== null (`self.Motion Controller`))
    (set `self.Motion Controller` null)
    (set `self.DraggedMesh` null)))

(fn `GetMoveTo`
  (params (`Neighbours List` :type "Array of PrimitiveComponent Object Reference"))
  (set `self.MoveToTarget` null)
  (for _array_element `Neighbours List`
    (if (not (`PrimitiveComponent.IsOverlappingActor` _array_element self))
      (set `self.MoveToTarget` _array_element)))
  (return))

(fn `GetNeightbours`
  (returns (Neightbours :type "Array of PrimitiveComponent Object Reference"))
  (bind _outcomponents (`KismetSystemLibrary.SphereOverlapComponents` (`SceneComponent.K2_GetComponentLocation` (`self.DraggedMesh`)) (`self.SphereRad`) (`|MakeArray` "ObjectTypeQuery1" "ObjectTypeQuery2" :!type "EObjectTypeQuery Enum") "/Script/Engine.BoxComponent"))
  (return _outcomponents))

(fn `IsSolved?`
  (returns (`Solved?` :type Boolean))
  (locals (Solve :type Boolean :default true))
  (for (_array_element _array_index) (`self.MeshTrackingList`)
    (if (not (`PrimitiveComponent.IsOverlappingComponent` _array_element (`|GetArrayItem` (`self.TrackingList`) _array_index)))
      (set `local.Solve` false)
      (break)))
  (return (`local.Solve`)))

(fn `ScalePuzzle`
  (`self.SetActorScale3D` (/ (1.0 1.0 1.0) (/ (* (`self.GridSize`) (`self.MeshSize`)) (`self.DesiredSize`))))
  (return))

(fn `ShufflePuzzle`
  (locals (Locations :type "Array of Vector Structure"))
  (bind _locations (`local.Locations`))
  (if (`self.Shuffled?`)
    (for _array_element (`self.TrackingList`)
      (`KismetArrayLibrary.Array_Add` (`local.Locations`) (`SceneComponent.RelativeLocation` _array_element)))
    (`KismetArrayLibrary.Array_Shuffle` (`local.Locations`))
    (for _array_element_2 (`self.MeshTrackingList`)
      (`SceneComponent.K2_SetRelativeLocation` _array_element_2 (`|GetArrayItem` _locations) false false)
      (`KismetArrayLibrary.Array_Remove` _locations))
    (return)
    (else
      (return))))

(fn `SpawnPuzzle`
  (bind _meshsize (`self.MeshSize`))
  (bind _meshsize_2 (`self.MeshSize`))
  (bind _trackinglist (`self.TrackingList`))
  (bind _meshtrackinglist (`self.MeshTrackingList`))
  (bind _returnvalue (`KismetMathLibrary.SafeDivide` (`self.MeshSize`) 4.0))
  (bind _returnvalue_2 (- (`self.GridSize`) 1))
  (bind _returnvalue_3 (- (`self.GridSize`) 1))
  (bind _returnvalue_4 (/ 1.0 (`KismetMathLibrary.Conv_IntToDouble` (`self.GridSize`))))
  ;[1 1 1] Delete Old
  (bind (_arrayindex _arrayelement) (`/Engine/EditorBlueprintResources/StandardMacros.ReverseForEachLoop` _trackinglist)
    (:`LoopBody`
      (`ActorComponent.K2_DestroyComponent` _arrayelement))
    (:`Completed`
      (`KismetArrayLibrary.Array_Clear` _trackinglist)
      (bind (_arrayindex_2 _arrayelement_2) (`/Engine/EditorBlueprintResources/StandardMacros.ReverseForEachLoop` _meshtrackinglist)
        (:`LoopBody`
          (`ActorComponent.K2_DestroyComponent` _arrayelement_2))
        (:`Completed`
          (`KismetArrayLibrary.Array_Clear` _meshtrackinglist)
          (for _index (range (+ _returnvalue_3 1))
            (set `self.Y-Variable` _index)
            (for _index_2 (range (+ _returnvalue_3 1))
              (set `self.X-Variable` _index_2)
              ;[1 1 1] Create Space
              (bind _returnvalue_5 (`AddComponent|NODE_AddBoxComponent-0` :`RelativeTransform` (`KismetMathLibrary.MakeTransform` (`KismetMathLibrary.MakeVector` (* (`self.X-Variable`) _meshsize) (* (`self.Y-Variable`) _meshsize)))))
              (`BoxComponent.SetBoxExtent` _returnvalue_5 (`KismetMathLibrary.MakeVector` _returnvalue _returnvalue _returnvalue) true)
              ;[1 1 1] Create Mesh
              (`PrimitiveComponent.SetCollisionObjectType` _returnvalue_5 "ECC_WorldDynamic")
              (`KismetArrayLibrary.Array_Add` (`self.TrackingList`) _returnvalue_5)
              (if (not (and (== (`self.Y-Variable`) _returnvalue_2) (== (`self.X-Variable`) _returnvalue_2)))
                (bind _returnvalue_6 (`AddComponent|NODE_AddStaticMeshComponent-0` :`RelativeTransform` (`KismetMathLibrary.MakeTransform` (`KismetMathLibrary.MakeVector` (* (`self.X-Variable`) _meshsize_2) (* (`self.Y-Variable`) _meshsize_2)))))
                (`SceneComponent.SetMobility` _returnvalue_6 "Movable")
                ;[1 1 1] Texture
                (`KismetArrayLibrary.Array_Add` (`self.MeshTrackingList`) _returnvalue_6)
                (bind _returnvalue_7 (`PrimitiveComponent.CreateDynamicMaterialInstance` _returnvalue_6 0 "/Game/Eigenarbeit/Assets/Stuff/Puzzle/PuzzleMaterial.PuzzleMaterial" "None"))
                (`MaterialInstanceDynamic.SetTextureParameterValue` _returnvalue_7 "PuzzleTexture" (`self.Texture`))
                (`MeshComponent.SetVectorParameterValueOnMaterials` _returnvalue_6 "TexOffset" (`KismetMathLibrary.MakeVector` (* (`self.X-Variable`) _returnvalue_4) (* (`self.Y-Variable`) _returnvalue_4) (* _returnvalue_4 (* (`self.GridSize`) (`self.GridSize`)))))
                (`|AddComponentByClass` "/Game/VRTemplate/Blueprints/GrabComponent.GrabComponent_C"))))
          (return))))))

(fn `UserConstructionScript`
  (`self.SpawnPuzzle`)
  (`self.ShufflePuzzle`)
  (`self.ScalePuzzle`))