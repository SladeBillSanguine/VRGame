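; VR sliding-tile puzzle actor that sets a linked Drawer's locked state from its solved check after a move.
; Construction script builds a grid of box slots and textured tiles with one gap, offsets each tile's texture, randomly shuffles and scales to DesiredSize.
; Grab line-traces for a tile, sphere-overlaps nearby slots for a free one, and constrains motion-controller dragging to that segment.
; IsSolved compares each tile's overlap with its same-index slot.
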(event `self.ReceiveTick`
  (params (DeltaSeconds :type "Float (single-precision)")))

(event `self.ReceiveBeginPlay`
  ;[1 1 1] Herausfinden des Targets
)

(event `/Game/Eigenarbeit/BP/GrabInterface.Grab`
  (params (MotionController :type "MotionControllerComponent Object Reference"))
  ;[1 1 1] Herausfinden des Targets
  (set `self.Motion Controller` MotionController)
  (bind _motioncontrollerdata (`HeadMountedDisplayFunctionLibrary.GetMotionControllerData` null "AnyHand"))
  (bind (_outhit _returnvalue) (`KismetSystemLibrary.LineTraceSingleForObjects` (`.AimPosition` (break `XRMotionControllerData` _motioncontrollerdata)) (+ (`.AimPosition` (break `XRMotionControllerData` _motioncontrollerdata)) (0.0 0.0 0.0)) (`|MakeArray` "ObjectTypeQuery2" :!type "EObjectTypeQuery Enum")))
  (if _returnvalue
    (for _array_element (`self.MeshTrackingList`)
      (if (== (`.HitComponent` (`GameplayStatics.BreakHitResult` _outhit)) _array_element)
        (if (not (`self.Is Being Grabbed`))
          (set `self.DraggedMesh` _array_element)
          (`self.MeshGrabbed`))))))

(event `MeshGrabbed`
  (set `self.DraggedMesh` null)
  (bind _neightbours (`self.GetNeightbours`))
  (`self.GetMoveTo` _neightbours)
  (`/Engine/EditorBlueprintResources/StandardMacros.IsValid` (`self.MoveToTarget`)
    (:`Is Valid`
      (`self.TriggeredMove`))))

(event `/Game/Eigenarbeit/BP/GrabInterface.Release`
  (params (MotionController :type "MotionControllerComponent Object Reference"))
  (if (== MotionController (`self.Motion Controller`))
    (set `self.Motion Controller` null)))

(event `TriggeredMove`
  (bind _motion_controller (`self.Motion Controller`) ; Not to Overlap
    (:`then`
      (set `self.Is Being Grabbed` true)
      (bind _output_get (set `self.MoveToStart` (`SceneComponent.RelativeLocation` (`self.DraggedMesh`))))
      (`SceneComponent.K2_SetRelativeLocation` (`self.DraggedMesh`) (`KismetMathLibrary.FindClosestPointOnSegment` (`SceneComponent.K2_GetComponentLocation` _motion_controller) _output_get (`SceneComponent.RelativeLocation` (`self.MoveToTarget`))) false false)
      (while (!= (`SceneComponent.RelativeLocation` (`self.DraggedMesh`)) (`SceneComponent.RelativeLocation` (`self.MoveToTarget`)))
        _)
      (set `self.Is Being Grabbed` false)
      (bind _solved_ (`self.IsSolved?`))
      (bind _asdrawer (cast `/Game/Eigenarbeit/BP/Drawer` (`self.Actor`)))
      (`/Game/Eigenarbeit/BP/Drawer.Set Locked State` _asdrawer _solved_))
    (:`else`)))

(fn `GetMoveTo`
  (params (`Neighbours List` :type "Array of PrimitiveComponent Object Reference"))
  (set `self.MoveToTarget` null)
  (for _array_element `Neighbours List`
    (if (not (`PrimitiveComponent.IsOverlappingActor` _array_element self))
      (set `self.MoveToTarget` _array_element)))
  (return))

(fn `GetNeightbours`
  (returns (Neightbours :type "Array of PrimitiveComponent Object Reference"))
  (bind _outcomponents (`KismetSystemLibrary.SphereOverlapComponents` (`SceneComponent.K2_GetComponentLocation` (`self.DraggedMesh`)) (`self.MeshSize`) (`|MakeArray` "ObjectTypeQuery1" "ObjectTypeQuery2" :!type "EObjectTypeQuery Enum") "/Script/Engine.BoxComponent"))
  (return _outcomponents))

(fn `IsSolved?`
  (returns (`Solved?` :type Boolean))
  (locals (Solve :type Boolean :default true))
  (for (_array_element _array_index) (`self.MeshTrackingList`)
    (if (not (`PrimitiveComponent.IsOverlappingComponent` _array_element (`|GetArrayItem` (`self.TrackingList`) _array_index)))
      (set `local.Solve` false)
      (break)))
  (return (`local.Solve`)))

(fn `ScalePuzzle`
  (`self.SetActorScale3D` (/ (1.0 1.0 1.0) (/ (* (`self.GridSize`) (`self.MeshSize`)) (`self.DesiredSize`))))
  (return))

(fn `ShufflePuzzle`
  (locals (Locations :type "Array of Vector Structure"))
  (bind _locations (`local.Locations`))
  (if (`self.Shuffled?`)
    (for _array_element (`self.TrackingList`)
      (`KismetArrayLibrary.Array_Add` (`local.Locations`) (`SceneComponent.RelativeLocation` _array_element)))
    (`KismetArrayLibrary.Array_Shuffle` (`local.Locations`))
    (for _array_element_2 (`self.MeshTrackingList`)
      (`SceneComponent.K2_SetRelativeLocation` _array_element_2 (`|GetArrayItem` _locations) false false)
      (`KismetArrayLibrary.Array_Remove` _locations))
    (return)
    (else
      (return))))

(fn `SpawnPuzzle`
  (bind _trackinglist (`self.TrackingList`))
  (bind _meshtrackinglist (`self.MeshTrackingList`))
  (bind _meshsize (`self.MeshSize`))
  (bind _meshsize_2 (`self.MeshSize`))
  (bind _returnvalue (`KismetMathLibrary.SafeDivide` (`self.MeshSize`) 4.0))
  (bind _returnvalue_2 (- (`self.GridSize`) 1))
  (bind _returnvalue_3 (- (`self.GridSize`) 1))
  (bind _returnvalue_4 (/ 1.0 (`KismetMathLibrary.Conv_IntToDouble` (`self.GridSize`))))
  ;[1 1 1] Delete Old
  (bind (_arrayindex _arrayelement) (`/Engine/EditorBlueprintResources/StandardMacros.ReverseForEachLoop` _trackinglist)
    (:`LoopBody`
      (`ActorComponent.K2_DestroyComponent` _arrayelement))
    (:`Completed`
      (`KismetArrayLibrary.Array_Clear` _trackinglist)
      (bind (_arrayindex_2 _arrayelement_2) (`/Engine/EditorBlueprintResources/StandardMacros.ReverseForEachLoop` _meshtrackinglist)
        (:`LoopBody`
          (`ActorComponent.K2_DestroyComponent` _arrayelement_2))
        (:`Completed`
          (`KismetArrayLibrary.Array_Clear` _meshtrackinglist)
          (for _index (range (+ _returnvalue_2 1))
            (set `self.Y-Variable` _index)
            (for _index_2 (range (+ _returnvalue_2 1))
              (set `self.X-Variable` _index_2)
              ;[1 1 1] Create Space
              (bind _returnvalue_5 (`AddComponent|NODE_AddBoxComponent-0` :`RelativeTransform` (`KismetMathLibrary.MakeTransform` (`KismetMathLibrary.MakeVector` (* (`self.X-Variable`) _meshsize_2) (* (`self.Y-Variable`) _meshsize_2)))))
              (`BoxComponent.SetBoxExtent` _returnvalue_5 (`KismetMathLibrary.MakeVector` _returnvalue _returnvalue _returnvalue) true)
              ;[1 1 1] Create Mesh
              (`KismetArrayLibrary.Array_Add` (`self.TrackingList`) _returnvalue_5)
              (if (not (and (== (`self.Y-Variable`) _returnvalue_3) (== (`self.X-Variable`) _returnvalue_3)))
                (bind _returnvalue_6 (`AddComponent|NODE_AddStaticMeshComponent-0` :`RelativeTransform` (`KismetMathLibrary.MakeTransform` (`KismetMathLibrary.MakeVector` (* (`self.X-Variable`) _meshsize) (* (`self.Y-Variable`) _meshsize)))))
                ;[1 1 1] Texture
                (`KismetArrayLibrary.Array_Add` (`self.MeshTrackingList`) _returnvalue_6)
                (bind _returnvalue_7 (`PrimitiveComponent.CreateDynamicMaterialInstance` _returnvalue_6 0 "/Game/Eigenarbeit/Assets/Stuff/Puzzle/PuzzleMaterial.PuzzleMaterial" "None"))
                (`MaterialInstanceDynamic.SetTextureParameterValue` _returnvalue_7 "PuzzleTexture" (`self.Texture`))
                (`MeshComponent.SetVectorParameterValueOnMaterials` _returnvalue_6 "TexOffset" (`KismetMathLibrary.MakeVector` (* (`self.X-Variable`) _returnvalue_4) (* (`self.Y-Variable`) _returnvalue_4) (* _returnvalue_4 (* (`self.GridSize`) (`self.GridSize`))))))))
          (return))))))

(fn `UserConstructionScript`
  (`self.SpawnPuzzle`)
  (set `self.Shuffled?` true)
  (`self.ShufflePuzzle`)
  (`self.ScalePuzzle`))