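; BP_SlidePuzzle is an actor that builds the board for a sliding tile puzzle at BeginPlay.
; SpawnPuzzle loops over a GridSize square, adding a box component at each MeshSize-spaced cell and storing it in TrackingList.
; Every cell except the last corner also gets a static mesh tile, leaving one gap.
; It holds only this setup, with no tile movement or win check.
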(event `self.ReceiveBeginPlay`
  (`self.SpawnPuzzle`))

(fn `SpawnPuzzle`
  (bind _meshsize (`self.MeshSize`))
  (bind _meshsize_2 (`self.MeshSize`))
  (bind _returnvalue (`KismetMathLibrary.SafeDivide` (`self.MeshSize`) 4.0))
  (bind _returnvalue_2 (- (`self.GridSize`) 1))
  (bind _returnvalue_3 (- (`self.GridSize`) 1))
  (for _index (range (+ _returnvalue_2 1))
    (set `self.Y-Variable` _index)
    (for _index_2 (range (+ _returnvalue_2 1))
      (set `self.X-Variable` _index_2)
      (bind _returnvalue_4 (`AddComponent|NODE_AddBoxComponent-0` :`RelativeTransform` (`KismetMathLibrary.MakeTransform` (`KismetMathLibrary.MakeVector` (* (`self.X-Variable`) _meshsize_2) (* (`self.Y-Variable`) _meshsize_2)))))
      (`BoxComponent.SetBoxExtent` _returnvalue_4 (`KismetMathLibrary.MakeVector` _returnvalue _returnvalue _returnvalue) true)
      (`KismetArrayLibrary.Array_Add` (`self.TrackingList`) _returnvalue_4)
      (if (not (and (== (`self.Y-Variable`) _returnvalue_3) (== (`self.X-Variable`) _returnvalue_3)))
        (`AddComponent|NODE_AddStaticMeshComponent-0` :`RelativeTransform` (`KismetMathLibrary.MakeTransform` (`KismetMathLibrary.MakeVector` (* (`self.X-Variable`) _meshsize) (* (`self.Y-Variable`) _meshsize))))))))

(fn `UserConstructionScript`)